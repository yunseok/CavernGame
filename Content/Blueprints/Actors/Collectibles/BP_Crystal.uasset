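; Collectible crystal that animates into the player on overlap and then destroys itself.
; When the player enters the sphere collision, it stores its location, scale and light intensity, then plays a timeline.
; Timeline curves lerp it toward the player's current position while shrinking it and fading its point light.
; Each timeline update also sets Score to the count of all crystals in the level plus one.
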(event OnComponentBeginOverlap(SphereCollisionComponent)
  (params (OverlappedComponent :type Primitive%20Component%20Object%20Reference) (OtherActor :type Actor%20Object%20Reference) (OtherComp :type Primitive%20Component%20Object%20Reference) (OtherBodyIndex :type Integer) (bFromSweep :type Boolean) (SweepResult :type Hit%20Result%20Structure%20%28by%20ref%29))
  (Utilities|IsPlayer OtherActor
    (:Is%20Player
      (CallFunction|StoreStartingValues)
      (bind (_direction _collection_progress _scale_progress _light_intensity) (Timeline|Collection%20Timeline Play)
        (:Update
          (CallFunction|MovetoPlayer _collection_progress (Game|Player|GetPlayerPawn 0))
          (CallFunction|ScaleCrystal _scale_progress)
          (CallFunction|SetLightIntensity _light_intensity)
          (bind _outactors (Actor|GetAllActorsOfClass "BP_Crystal_C"))
          (Variables|Default|SetScore (+ (Utilities|Array|Length _outactors) 1)))
        (:Finished
          (Actor|DestroyActor))))))

(fn ConstructionScript)

(fn MovetoPlayer
  (params (Alpha :type Float%20%28single-precision%29) (self2 :type Actor%20Object%20Reference))
  (Transformation|SetActorLocation (Math|Vector|Lerp(Vector) (Variables|Default|GetStarting%20Location) (Transformation|GetActorLocation self2) Alpha) false false))

(fn StoreStartingValues
  (Variables|Default|SetStarting%20Location (Transformation|GetActorLocation))
  (Variables|Default|SetStarting%20Scale (Transformation|GetActorScale3D))
  (Variables|Default|SetStarting%20Light%20Intensity (Variables|/Script/Engine.LightComponentBase|GetIntensity (Variables|Default|GetPointLight))))

(fn ScaleCrystal
  (params (Alpha :type Float%20%28single-precision%29))
  (Transformation|SetActorScale3D (Math|Vector|Lerp(Vector) (Variables|Default|GetStarting%20Scale) "0, 0, 0" Alpha)))

(fn SetLightIntensity
  (params (Alpha :type Float%20%28single-precision%29))
  (Rendering|Components|Light|SetIntensity (Variables|Default|GetPointLight) (Math|Float|Lerp (Variables|Default|GetStarting%20Light%20Intensity) 0.0 Alpha)))