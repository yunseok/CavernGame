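; BP_TriggerDeath is a death trigger volume that restarts the current level when the player touches it.
; On BeginPlay it fades the camera in from white, so each reload opens smoothly.
; When the first player pawn overlaps the Trigger component, it fades the screen to white, waits briefly, then reopens the current level by name.
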(event OnComponentBeginOverlap(Trigger)
  (params (OverlappedComponent :type Primitive%20Component%20Object%20Reference) (OtherActor :type Actor%20Object%20Reference) (OtherComp :type Primitive%20Component%20Object%20Reference) (OtherBodyIndex :type Integer) (bFromSweep :type Boolean) (SweepResult :type Hit%20Result%20Structure%20%28by%20ref%29))
  (if (== OtherActor (Game|Player|GetPlayerPawn 0))
    (CameraFades|StartCameraFade (Game|GetPlayerCameraManager 0) 0.0 1.0 0.25 "(R=1.000000,G=1.000000,B=1.000000,A=1.000000)" false true)
    (Utilities|FlowControl|Delay 0.5)
    (bind _returnvalue (Game|GetCurrentLevelName true))
    (Game|OpenLevel(byName) (Utilities|String|StringToName _returnvalue))))

(event EventBeginPlay
  (CameraFades|StartCameraFade (Game|GetPlayerCameraManager 0) 1.0 0.0 0.25 "(R=1.000000,G=1.000000,B=1.000000,A=1.000000)" false true))

(event Collision|EventActorBeginOverlap
  (params (OtherActor :type Actor%20Object%20Reference)))

(event EventTick
  (params (DeltaSeconds :type Float%20%28single-precision%29)))

(fn ConstructionScript)