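; BP_TriggerWin is a level-end trigger actor that reacts to player overlap and checks whether any BP_Crystal actors remain.
; It finds the current level in a LevelNames array to detect the final level; CompleteLevel calls a same-named CompleteLevel when the level is not final.
; The overlap branch currently takes no action after the crystal check, and LoadNextLevel is empty.
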(event Collision|EventActorBeginOverlap
  (params (OtherActor :type Actor%20Object%20Reference))
  (Utilities|IsPlayer OtherActor
    (:Is%20Player
      (if (CallFunction|AnyCrystalsRemaining)
        _))))

(fn ConstructionScript)

(fn AnyCrystalsRemaining
  (bind _outactors (Actor|GetAllActorsOfClass "/Game/Blueprints/Actors/Collectibles/BP_Crystal.BP_Crystal_C"))
  (return (> (Utilities|Array|Length _outactors) 0)))

(fn CompleteLevel
  (if (not (CallFunction|IsFinalLevel))
    (CallFunction|CompleteLevel)))

(fn GetCurrentLevelIndex
  (bind _returnvalue (Game|GetCurrentLevelName true))
  (return (Utilities|Array|FindItem (Variables|Default|GetLevel%20Names) (Utilities|String|StringToName _returnvalue))))

(fn IsFinalLevel
  (return (== (Utilities|Array|LastIndex (Variables|Default|GetLevel%20Names)) (CallFunction|GetCurrentLevelIndex))))

(fn LoadNextLevel)