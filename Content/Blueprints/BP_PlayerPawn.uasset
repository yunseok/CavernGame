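; BP_PlayerPawn is a player pawn that moves a physics Sphere by applying torque from input.
; Forward/backward and left/right axes apply torque around Y and X, scaled by AccelerationMultiplier and applied as an acceleration change, independent of mass.
; The Jump axis likewise applies torque around Z, so it spins the sphere about the vertical axis and adds no upward impulse.
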(event EventBeginPlay)

(event Collision|EventActorBeginOverlap
  (params (OtherActor :type Actor%20Object%20Reference)))

(event EventTick
  (params (DeltaSeconds :type Float%20%28single-precision%29)))

(event Input|AxisEvents|InputAxisMoveForward/Backward
  (params (AxisValue :type Float%20%28single-precision%29))
  (Class|PrimitiveComponent|AddTorqueinRadians (Variables|Default|GetSphere) (Math|Vector|MakeVector 0.0 (* AxisValue (Variables|Default|GetAcceleration%20Multiplier)) 0.0) "None" true))

(event Input|AxisEvents|InputAxisMoveLeft/Right
  (params (AxisValue :type Float%20%28single-precision%29))
  (Class|PrimitiveComponent|AddTorqueinRadians (Variables|Default|GetSphere) (Math|Vector|MakeVector (* AxisValue (Variables|Default|GetAcceleration%20Multiplier)) 0.0 0.0) "None" true))

(event Input|AxisEvents|InputAxisJump
  (params (AxisValue :type Float%20%28single-precision%29))
  (Class|PrimitiveComponent|AddTorqueinRadians (Variables|Default|GetSphere) (Math|Vector|MakeVector 0.0 0.0 (* AxisValue (Variables|Default|GetAcceleration%20Multiplier))) "None" true))

(fn ConstructionScript)